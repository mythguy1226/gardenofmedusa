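; BP_Medusa is the Medusa enemy, which wanders along a Pathfinder path and kills players it keeps in sight.
; Tick runs a Wandering/Pursuing/Attacking state switch, though Pursue is empty and nothing here changes the state.
; AI Perception sets or clears the player reference.
; While it is set, a countdown runs independently of state, triggering the player's death at zero; losing sight resets the timer.
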(event OnTargetPerceptionUpdated(AIPerception)
  (params (Actor :type Actor%20Object%20Reference) (Stimulus :type AI%20Stimulus%20Structure))
  ;[1 1 1] Check to see if we can see the player, if so set it to the player, if we break connection deref the player var and reset the timer
  (if (.bsuccessfullysensed Stimulus)
    (bind _asbp_first_person_character (Utilities|Casting|CastToBP_FirstPersonCharacter Actor))
    (Variables|Default|SetPlayer _asbp_first_person_character)
    (else
      (Variables|Default|SetPlayer 0)
      (Variables|Default|SetAttackTimer 3.0))))

(event Custom|Wander
  (Default|MoveAlongPath (Variables|Default|GetPathfinder)))

(event Custom|Pursue)

(event Custom|Attack
  ;[1 1 1] Check to see if there is a player, then call the player death function and reset the timer and deref the player
  (bind _player (Variables|Default|GetPlayer)
    (:then
      (Default|Death _player)
      (Variables|Default|SetAttackTimer 3.0)
      (Variables|Default|SetPlayer 0))
    (:else)))

(event EventBeginPlay
  (Default|SetTargetPath (Variables|Default|GetPathfinder) (Math|Conversions|ToVector(Vector2D) (Variables|Default|GetTarget))))

(event EventTick
  (params (DeltaSeconds :type Float%20%28single-precision%29))
  (Utilities|FlowControl|Sequence
    (:then_0
      ;[1 1 1] FSM for handling Medusa's behavior
      (switch Utilities|FlowControl|Switch|SwitchonMedusaStates (Variables|Default|GetCurrentState)
        (:NewEnumerator0
          (CallFunction|Wander))
        (:NewEnumerator1
          (CallFunction|Pursue))
        (:NewEnumerator2
          (CallFunction|Attack))))
    (:then_1
      ;[1 1 1] Check to ensure there is a player it is attacking, then reduce the attack timer. If the attack timer is <= 0, trigger the attack function
      (if (!= (Variables|Default|GetPlayer) 0)
        (Variables|Default|SetAttackTimer (- (Variables|Default|GetAttackTimer) (Utilities|Time|GetWorldDeltaSeconds)))
        (if (<= (Variables|Default|GetAttackTimer) 0.0)
          (CallFunction|Attack))))))

(fn ConstructionScript)