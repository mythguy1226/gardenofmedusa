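; Snake vassal sentry AI that watches for the player and alerts Medusa.
; A Tick-driven state machine alternates between Static, sweeping its view with a timeline on a countdown, and Wandering between two location actors via AI MoveTo.
; Sight perception stores the player and last seen location; spotting movement switches to Alerting, which redirects Medusa's pathfinder there once.
; Losing sight returns it to Static and re-arms the alert.
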(event OnTargetPerceptionUpdated(Sight)
  (params (Actor :type Actor%20Object%20Reference) (Stimulus :type AI%20Stimulus%20Structure))
  ;[1 1 1] Check to see if we can see the player, if so set it to the player, if we break connection deref the player var and reset the timer
  (if (.bsuccessfullysensed Stimulus)
    (bind _asbp_first_person_character (Utilities|Casting|CastToBP_FirstPersonCharacter Actor))
    (Variables|Default|Setplayer _asbp_first_person_character)
    (Variables|Default|SetlastSeenLocation (.stimuluslocation Stimulus))
    (else
      (Variables|Default|Setplayer 0))))

(event EventBeginPlay
  (Variables|Default|SetoriginalRotation (Transformation|GetActorRotation))
  (Variables|Default|SetOriginalLoc (Transformation|GetActorLocation)))

(event Collision|EventActorBeginOverlap
  (params (OtherActor :type Actor%20Object%20Reference)))

(event EventTick
  (params (DeltaSeconds :type Float%20%28single-precision%29))
  (switch Utilities|FlowControl|Switch|SwitchonVassalStates (Variables|Default|GetcurrentState)
    (:NewEnumerator0
      (bind _output_get (Variables|Default|SetlookTIme (- (Variables|Default|GetlookTIme) DeltaSeconds)))
      (if (<= _output_get 0.0)
        (Variables|Default|SetlookTIme 3.0)
        (Math|Float|IncrementFloat (Variables|Default|GetlookCount)
          (:%20%20
            ;[1 1 1] Have the snake vassal look from side to side every 3 seconds, after doing this 3 times, we will then tell the vassal to wander to the next location
            (if (< (Variables|Default|GetlookCount) 3.0)
              (Utilities|FlowControl|FlipFlop
                (:A
                  (Timeline|Timeline PlayFromStart
                    (:Update
                      (Transformation|SetActorRotation (Math|Interpolation|RInterpTo (Variables|Default|GetoriginalRotation) (Math|Rotator|MakeRotator 0.0 0.0 (+ (.yaw (Variables|Default|GetoriginalRotation)) 6e+01)) DeltaSeconds 2.0))
                      ;[1 1 1] If we see the player and they are moving, then set the alarm
                      (bind _player (Variables|Default|Getplayer :!label _label)
                        (:then
                          (if (Variables|/Game/FirstPerson/Blueprints/BP_FirstPersonCharacter.BP_FirstPersonCharacter_C|GetisMoving _player)
                            (Variables|Default|SetcurrentState "NewEnumerator2")))
                        (:else)))))
                (:B
                  (Timeline|Timeline ReverseFromEnd)))
              (else
                (Variables|Default|SetcurrentState "NewEnumerator1")
                (Variables|Default|SetlookCount 0.0)))))))
    (:NewEnumerator1
      ;[1 1 1] Move the vassal to the desired location, then have it go backwards
      (if (Variables|Default|Getforwards)
        (AI|AIMoveTo (Pawn|GetControlledPawn (AI|GetAIController self)) (Transformation|GetActorLocation (Variables|Default|GettargetLocActor)) 0 2e+01 true
          (:then
            (goto _label))
          (:OnSuccess
            (Variables|Default|Setforwards false)
            (Variables|Default|SetcurrentState "NewEnumerator0")))
        (else
          (AI|AIMoveTo (Pawn|GetControlledPawn (AI|GetAIController self)) (Transformation|GetActorLocation (Variables|Default|GetoriginalLocActor)) 0 2e+01 true
            (:then
              (goto _label))
            (:OnSuccess
              (Variables|Default|Setforwards true)
              (Variables|Default|SetcurrentState "NewEnumerator0")
              (Variables|Default|SetoriginalRotation (Transformation|GetActorRotation)))))))
    (:NewEnumerator2
      ;[1 1 1] When in alert mode, tell Medusa to change its path to where the player was last seen
      (Variables|Default|Getplayer
        (:then
          (bind _returnvalue (Actor|GetActorOfClass "/Game/GardenOfMedusa/Blueprints/Characters/BP_Medusa.BP_Medusa_C"))
          (Utilities|FlowControl|DoOnce false :!label _label_2
            (:Completed
              (Default|ChangePath (Variables|/Game/GardenOfMedusa/Blueprints/Characters/BP_Medusa.BP_Medusa_C|GetPathfinder _returnvalue) (Variables|Default|GetlastSeenLocation)))))
        (:else
          (Variables|Default|SetcurrentState "NewEnumerator0")
          (goto _label_2 Reset))))))

(fn ConstructionScript)