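; BP_StationaryVassal is a stationary snake vassal enemy that spits slowing venom at the player and alerts Medusa.
; An AI sight perception component caches the player when seen and, once per sighting, redirects Medusa's Pathfinder to the stimulus location.
; Tick checks perceived actors for the player, spawns BP_SlowingVenom aimed at them with a spit sound, then counts down a short cooldown before the next shot.
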(event OnTargetPerceptionUpdated(Sight)
  (params (Actor :type Actor%20Object%20Reference) (Stimulus :type AI%20Stimulus%20Structure))
  ;[1 1 1] Check to see if we can see the player, if so set it to the player, if we break connection deref the player var and reset the ability to change the path to the player
  (if (.bsuccessfullysensed Stimulus)
    (bind _asbp_first_person_character (Utilities|Casting|CastToBP_FirstPersonCharacter Actor))
    (Variables|Default|Setplayer _asbp_first_person_character)
    (Utilities|FlowControl|DoOnce false :!label _label
      (:Completed
        (bind _returnvalue (Actor|GetActorOfClass "/Game/GardenOfMedusa/Blueprints/Characters/BP_Medusa.BP_Medusa_C"))
        (Default|ChangePath (Variables|/Game/GardenOfMedusa/Blueprints/Characters/BP_Medusa.BP_Medusa_C|GetPathfinder _returnvalue) (.stimuluslocation Stimulus))))
    (else
      (Variables|Default|Setplayer 0)
      (goto _label Reset))))

(event EventBeginPlay)

(event Collision|EventActorBeginOverlap
  (params (OtherActor :type Actor%20Object%20Reference)))

(event EventTick
  (params (DeltaSeconds :type Float%20%28single-precision%29))
  (bind _returnvalue (Transformation|GetActorLocation))
  ;[1 1 1] Check to see if the vassal can shoot, if so continue, if not, give it a .5 second cooldown between shots
  (if (Variables|Default|GetcanShoot)
    ;[1 1 1] Loop through all perceived actors and if they are the player, then we will shoot at them and set it so the enemy cant shoot
    (for _array_element (Class|AIPerceptionComponent|GetPerceivedActors (Variables|Default|GetSight) "/Script/AIModule.AISense_Sight")
      (if (== _array_element (Variables|Default|Getplayer))
        (Game|SpawnActorfromClass "/Game/GardenOfMedusa/Blueprints/Characters/SnakeVassals/BP_SlowingVenom.BP_SlowingVenom_C" (Math|Transform|MakeTransform _returnvalue (Math|Rotator|FindLookatRotation _returnvalue (Transformation|GetActorLocation _array_element)) "1.000000,1.000000,1.000000") "AdjustIfPossibleButAlwaysSpawn" 0 0)
        (Audio|PlaySound2D "/Game/GardenOfMedusa/Assets/Sounds/VassalSpit.VassalSpit" 1.0 1.0 0.0 0 0)
        (Variables|Default|SetcanShoot false)))
    (elif (< (- (Variables|Default|GetshootTIme) DeltaSeconds) 0.0)
      (Variables|Default|SetcanShoot true)
      (Variables|Default|SetshootTIme 0.5)
      (else
        (Variables|Default|SetshootTIme (- (Variables|Default|GetshootTIme) DeltaSeconds))))))

(fn ConstructionScript)