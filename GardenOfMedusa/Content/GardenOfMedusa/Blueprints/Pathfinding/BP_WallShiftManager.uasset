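; Manager that periodically shifts BP_ShiftingWall actors in the level, favoring those near the player.
; On BeginPlay it gathers every wall, waits briefly, then starts a self-repeating ShiftWalls cycle paced by TimeBetweenShifts.
; Each cycle shifts random picks from the closest-walls list, then, after a short delay, random picks from all walls.
; GetClosestWalls draws on SortWallsArray, a bubble sort by distance to the player.
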(event Custom|ShiftWalls
  (bind _walls (Variables|Default|GetWalls))
  (bind _walls_2 (Variables|Default|GetWalls))
  (bind _returnvalue (Utilities|Array|Length _walls_2))
  (bind _returnvalue_2 (Math|Random|RandomInteger _returnvalue))
  (bind _output (Utilities|Array|Get(acopy) _walls _returnvalue_2))
  ;[1 1 1] Get the closest walls to the player and then shift them
  (bind _out_walls (CallFunction|GetClosestWalls 3))
  (for _index (range 0 2)
    (Utilities|IsValid (Utilities|Array|Get(acopy) _out_walls (Math|Random|RandomInteger (Utilities|Array|Length _out_walls)))
      (:Is%20Valid
        (Default|ShiftWall (Utilities|Array|Get(acopy) _out_walls (Math|Random|RandomInteger (Utilities|Array|Length _out_walls)))))))
  ;[1 1 1] Shift a couple random walls as well
  (Utilities|FlowControl|Delay 0.2)
  (for _index_2 (range 0 2)
    (Utilities|IsValid _output
      (:Is%20Valid
        (Default|ShiftWall _output))))
  ;[1 1 1] Call a wall shift again after delay is up
  (Utilities|FlowControl|Delay (Variables|Default|GetTimeBetweenShifts))
  (CallFunction|ShiftWalls))

(event EventBeginPlay
  ;[1 1 1] Get references to each shifting wall in the scene
  (bind _outactors (Actor|GetAllActorsOfClass "/Game/GardenOfMedusa/Blueprints/Pathfinding/MazeEnv/BP_ShiftingWall.BP_ShiftingWall_C"))
  (Variables|Default|SetWalls _outactors)
  ;[1 1 1] Initial wall shifting
  (Utilities|FlowControl|Delay 5.0)
  (CallFunction|ShiftWalls))

(fn ConstructionScript)

(fn SortWallsArray
  ;[1 1 1] Double loop to iterate through the array multiple times. This ensures multiple passes for sorting if needed
  (LocalVariables|SetSortedWalls (Variables|Default|GetWalls))
  (for _index (range 0 (- (Utilities|Array|Length (LocalVariables|GetSortedWalls)) 1))
    (LocalVariables|SetSwapped false)
    (for _index_2 (range 0 (- (- (Utilities|Array|Length (LocalVariables|GetSortedWalls)) _index) 1))
      ;[1 1 1] Set the checked indices
      (LocalVariables|SetCheckIndex _index_2)
      (LocalVariables|SetCheckNextIndex (Math|Integer|%(Integer) (+ _index_2 1) (Utilities|Array|Length (LocalVariables|GetSortedWalls))))
      (if (> (Math|Vector|Distance(Vector) (Transformation|GetActorLocation (Utilities|Array|Get(acopy) (LocalVariables|GetSortedWalls) (LocalVariables|GetCheckIndex))) (Transformation|GetActorLocation (Game|GetPlayerCharacter 0))) (Math|Vector|Distance(Vector) (Transformation|GetActorLocation (Utilities|Array|Get(acopy) (LocalVariables|GetSortedWalls) (LocalVariables|GetCheckNextIndex))) (Transformation|GetActorLocation (Game|GetPlayerCharacter 0))))
        ;[1 1 1] If wall is closer to player then swap
        (Utilities|Array|Swap (LocalVariables|GetSortedWalls) (LocalVariables|GetCheckIndex) (LocalVariables|GetCheckNextIndex))
        (LocalVariables|SetSwapped true))))
  ;[1 1 1] If one pass goes through and nothing was swapped, the array is now sorted and can be returned.
  (if (not (LocalVariables|GetSwapped))
    (return (LocalVariables|GetSortedWalls))))

(fn GetClosestWalls
  (params (Num%20Walls :type Integer))
  ;[1 1 1] Transfer the closest walls to the player from the sorted walls array
  (bind _out_walls (CallFunction|SortWallsArray))
  (LocalVariables|SetSortedWalls _out_walls)
  (for _index (range 0 Num%20Walls)
    (Utilities|Array|AddUnique (LocalVariables|GetClosestWalls) (Utilities|Array|Get(acopy) (LocalVariables|GetSortedWalls) _index)))
  (return (LocalVariables|GetClosestWalls)))