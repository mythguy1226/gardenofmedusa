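; Pathfinder component that finds and follows paths across a node grid for its owning character, with re-pathing support for BP_Medusa.
; It runs A* on a worker thread using a priority-queue open set, weighted node costs, eight-way neighbors and a Manhattan heuristic.
; MoveAlongPath feeds movement input and facing from the stored path.
; UpdateDynamicNodes syncs changed grid costs and re-paths, while a recursive helper picks random navigable points.
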(event Custom|Change%20Path
  (params (Target :type Vector))
  ;[1 1 1] Set the path from the actor's position to the target position
  (if (not (Variables|Default|GetCalculatingPath))
    (|MultiThreadedNode
      (:MultiThreadedWork
        (Variables|Default|SetCalculatingPath true)
        (Pathfinding|FindPathtoTarget (.gridindex (Default|GetNodefromWorldPosition (Variables|Default|GetGrid) (Math|Conversions|ToVector2D(Vector) (Transformation|GetActorLocation (Components|GetOwner))))) (.gridindex (Default|GetNodefromWorldPosition (Variables|Default|GetGrid) (Math|Conversions|ToVector2D(Vector) Target)))))
      (:FinishedWork
        (Variables|Default|SetCalculatingPath false)
        ;[1 1 1] Highlight path when in debug mode
        (if (Variables|Default|GetDebugMode)
          (Rendering|Debug|FlushPersistentDebugLines)
          (Debug|HighlightCurrentPath))))))

(event EventBeginPlay
  ;[1 1 1] Set the nodes as reference to nodes from grid
  (Variables|Default|SetNodes (Variables|/Game/GardenOfMedusa/Blueprints/Pathfinding/BP_Grid.BP_Grid_C|GetNodes (Variables|Default|GetGrid))))

(event EventTick
  (params (DeltaSeconds :type Float%20%28single-precision%29)))

(fn GetNodeNeighbors
  (params (Grid%20Index :type Vector%202D%20Structure))
  ;[1 1 1] Iterate through all potential neighbors
  (bind _output_get (LocalVariables|SetPossible%20Neighbors (Utilities|Array|MakeArray "(X=1.000000,Y=0.000000)" "(X=0.000000,Y=1.000000)" "(X=-1.000000,Y=0.000000)" "(X=0.000000,Y=-1.000000)" "(X=1.000000,Y=1.000000)" "(X=-1.000000,Y=-1.000000)" "(X=1.000000,Y=-1.000000)" "(X=-1.000000,Y=1.000000)")))
  (for _array_element _output_get
    ;[1 1 1] Check if the potential node is walkable or not and add to the neighbors list if it is
    (if (.ReturnValue (Utilities|Map|Find (Variables|Default|GetNodes) (+ _array_element Grid%20Index)))
      (if (and (Utilities|Enum|NotEqual(Enum) (.groundtype (.Value (Utilities|Map|Find (Variables|Default|GetNodes) (+ _array_element Grid%20Index)))) "NewEnumerator4") (Utilities|Enum|NotEqual(Enum) (.groundtype (.Value (Utilities|Map|Find (Variables|Default|GetNodes) (+ _array_element Grid%20Index)))) "NewEnumerator3"))
        (if (Math|Boolean|NANDBoolean (Utilities|Enum|Equal(Enum) (.groundtype (.Value (Utilities|Map|Find (Variables|Default|GetNodes) (+ _array_element Grid%20Index)))) "NewEnumerator5") (== (.nodecost (.Value (Utilities|Map|Find (Variables|Default|GetNodes) (+ _array_element Grid%20Index)))) 9999))
          (Utilities|Array|AddUnique (LocalVariables|GetOut%20Neighbors) (+ _array_element Grid%20Index))))))
  (return (LocalVariables|GetOut%20Neighbors)))

(fn GetEstimatedCosttoTarget
  (params (currentNode :type Vector%202D%20Structure) (targetNode :type Vector%202D%20Structure))
  (bind _returnvalue (- currentNode targetNode))
  (return (Math|Float|Round (+ (Math|Float|Absolute(Float) (.x _returnvalue)) (Math|Float|Absolute(Float) (.y _returnvalue))))))

(fn RetracePath
  (params (Start%20Node :type Vector%202D%20Structure) (Target%20Node :type Vector%202D%20Structure))
  ;[1 1 1] Set start node as current and loop until you've found the end
  (LocalVariables|SetCurrentNode Start%20Node)
  (while (Utilities|Operators|NotEqual(!=) (LocalVariables|GetCurrentNode) Target%20Node 0.0001)
    ;[1 1 1] Add current node to reversed path and set that node's previous as the current node
    (Utilities|Array|AddUnique (LocalVariables|GetReversed%20Path) (LocalVariables|GetCurrentNode))
    (LocalVariables|SetCurrentNode (.previousnode (.Value (Utilities|Map|Find (Variables|Default|GetNodes) (LocalVariables|GetCurrentNode))))))
  ;[1 1 1] Iterate through loop backwards to reverse path. Then store in output path
  (bind _arrayelement (Utilities|Array|ReverseforEachLoop (LocalVariables|GetReversed%20Path))
    (:LoopBody
      (Utilities|Array|AddUnique (LocalVariables|GetOut%20Path) _arrayelement))
    (:Completed
      (return (LocalVariables|GetOut%20Path)))))

(fn FindPathtoTarget
  (params (Start%20Position :type Vector%202D%20Structure) (Target%20Position :type Vector%202D%20Structure))
  (bind _nodes (Variables|Default|GetNodes))
  (bind _nodes_2 (Variables|Default|GetNodes))
  (bind _nodes_3 (Variables|Default|GetNodes))
  ;[1 1 1] Set the start and target nodes. Also check if the target node is within the grid
  (LocalVariables|SetStart%20Node%20L Start%20Position)
  (LocalVariables|SetTarget%20Node%20L Target%20Position)
  (if (Math|Boolean|ANDBoolean (Utilities|Enum|NotEqual(Enum) (.groundtype (.Value (Utilities|Map|Find (Variables|Default|GetNodes) (LocalVariables|GetTarget%20Node%20L)))) "NewEnumerator4") (Utilities|Enum|NotEqual(Enum) (.groundtype (.Value (Utilities|Map|Find (Variables|Default|GetNodes) (LocalVariables|GetTarget%20Node%20L)))) "NewEnumerator3") (.ReturnValue (Utilities|Map|Find (Variables|Default|GetNodes) (LocalVariables|GetTarget%20Node%20L))))
    (Utilities|FlowControl|Sequence
      (:then_0
        ;[1 1 1] Set default values
        (bind _keys (Utilities|Map|Keys (Variables|Default|GetNodes)))
        (for _array_element _keys
          (Utilities|Map|Add _nodes_2 _array_element (Utilities|Struct|MakeStruct_Node (.groundtype (.Value (Utilities|Map|Find _nodes_2 _array_element))) (.worldlocation (.Value (Utilities|Map|Find _nodes_2 _array_element))) (.gridindex (.Value (Utilities|Map|Find _nodes_2 _array_element))) (.nodecost (.Value (Utilities|Map|Find _nodes_2 _array_element))) 999 999 999 "(X=0.000000,Y=0.000000)")))
        (Utilities|Map|Add _nodes (LocalVariables|GetStart%20Node%20L) (Utilities|Struct|MakeStruct_Node (.groundtype (.Value (Utilities|Map|Find _nodes (LocalVariables|GetStart%20Node%20L)))) (.worldlocation (.Value (Utilities|Map|Find _nodes (LocalVariables|GetStart%20Node%20L)))) (.gridindex (.Value (Utilities|Map|Find _nodes (LocalVariables|GetStart%20Node%20L)))) (.nodecost (.Value (Utilities|Map|Find _nodes (LocalVariables|GetStart%20Node%20L)))) (Pathfinding|GetEstimatedCosttoTarget (LocalVariables|GetStart%20Node%20L) (LocalVariables|GetTarget%20Node%20L)) 0 (Pathfinding|GetEstimatedCosttoTarget (LocalVariables|GetStart%20Node%20L) (LocalVariables|GetTarget%20Node%20L)) "(X=0.000000,Y=0.000000)")))
      (:then_1
        ;[1 1 1] Set current node to start node and add it to the open set
        (LocalVariables|SetCurrentNode (LocalVariables|GetStart%20Node%20L))
        (bind _out_queue (CallFunction|Push (LocalVariables|GetNewOpenSet) (LocalVariables|GetStart%20Node%20L) (Variables|Default|GetGrid)))
        (LocalVariables|SetNewOpenSet _out_queue)
        ;[1 1 1] Loop as long as there are elements in the open set
        (while (not (CallFunction|IsEmpty (LocalVariables|GetNewOpenSet)))
          ;[1 1 1] Set the new cheapest node to be the current, remove it from the open set, and finally add it to the closed set
          (bind (_out_node _out_queue_2) (CallFunction|Pop (LocalVariables|GetNewOpenSet)))
          (LocalVariables|SetNewOpenSet _out_queue_2)
          (LocalVariables|SetCurrentNode _out_node)
          (Utilities|Array|AddUnique (LocalVariables|GetClosedSet) (LocalVariables|GetCurrentNode))
          ;[1 1 1] Get the current node's neighbors and iterate through them
          (for _array_element_2 (Pathfinding|GetNodeNeighbors (LocalVariables|GetCurrentNode))
            (LocalVariables|SetCurrentNeighbor _array_element_2)
            ;[1 1 1] Check if the current neighbor is in the closed set. If it isn't proceed.
            (if (not (Utilities|Array|ContainsItem (LocalVariables|GetClosedSet) (LocalVariables|GetCurrentNeighbor)))
              ;[1 1 1] Calculate and set the current neighbor's cost from start
              (LocalVariables|SetCurrentNeighborCostFromStart (+ (.costfromstart (.Value (Utilities|Map|Find (Variables|Default|GetNodes) (LocalVariables|GetCurrentNode)))) (.nodecost (.Value (Utilities|Map|Find (Variables|Default|GetNodes) (LocalVariables|GetCurrentNeighbor))))))
              ;[1 1 1] Check if the current neighbor is in the open set. If it isn't, add it. If it is, check its costs
              (if (not (Utilities|Array|ContainsItem (.nodearray (LocalVariables|GetNewOpenSet)) (LocalVariables|GetCurrentNeighbor)))
                (bind _out_queue_3 (CallFunction|Push (LocalVariables|GetNewOpenSet) (LocalVariables|GetCurrentNeighbor) (Variables|Default|GetGrid)))
                (LocalVariables|SetNewOpenSet _out_queue_3)
                ;[1 1 1] Set new cost values of neighbors of the current node
                (Utilities|Map|Add _nodes_3 (LocalVariables|GetCurrentNeighbor) (Utilities|Struct|MakeStruct_Node (.groundtype (.Value (Utilities|Map|Find _nodes_3 (LocalVariables|GetCurrentNeighbor)))) (.worldlocation (.Value (Utilities|Map|Find _nodes_3 (LocalVariables|GetCurrentNeighbor)))) (.gridindex (.Value (Utilities|Map|Find _nodes_3 (LocalVariables|GetCurrentNeighbor)))) (.nodecost (.Value (Utilities|Map|Find _nodes_3 (LocalVariables|GetCurrentNeighbor)))) (+ (LocalVariables|GetCurrentNeighborCostFromStart) (Pathfinding|GetEstimatedCosttoTarget (LocalVariables|GetCurrentNeighbor) (LocalVariables|GetTarget%20Node%20L))) (LocalVariables|GetCurrentNeighborCostFromStart) (Pathfinding|GetEstimatedCosttoTarget (LocalVariables|GetCurrentNeighbor) (LocalVariables|GetTarget%20Node%20L)) (LocalVariables|GetCurrentNode)) :!label _label)
                ;[1 1 1] Once you've found the target node, retrace the path and store it
                (if (Utilities|Operators|EqualEqual (LocalVariables|GetCurrentNeighbor) (LocalVariables|GetTarget%20Node%20L) 0.0001)
                  (Variables|Default|SetPath (Pathfinding|RetracePath (LocalVariables|GetTarget%20Node%20L) (LocalVariables|GetStart%20Node%20L)))
                  (return))
                (elif (< (LocalVariables|GetCurrentNeighborCostFromStart) (.costfromstart (.Value (Utilities|Map|Find _nodes_3 (LocalVariables|GetCurrentNeighbor)))))
                  (goto _label))))))
        ;[1 1 1] Unable to get path
        (return)))))

(fn HighlightCurrentPath
  (Class|KismetSystemLibrary|FlushDebugStrings)
  ;[1 1 1] Iterate through each node in the path and highlight it
  (for _array_element (Variables|Default|GetPath)
    (Rendering|Debug|DrawDebugSphere (.worldlocation (.Value (Utilities|Map|Find (Variables|Default|GetNodes) _array_element))) 5e+01 12 "(R=0.000000,G=0.918137,B=1.000000,A=1.000000)" 5e+01 1.0)))

(fn MoveAlongPath
  (bind _returnvalue (Components|GetOwner))
  (bind _path (Variables|Default|GetPath))
  (bind _nodes (Variables|Default|GetNodes))
  (bind _output (Utilities|Array|Get(acopy) _path))
  (bind _value (Utilities|Map|Find _nodes _output))
  ;[1 1 1] Move along path if a path exists
  (if (> (Utilities|Array|Length (Variables|Default|GetPath)) 0)
    ;[1 1 1] Calculate the direction to the first node in the path, apply movement input to the character, and turn to face the move direction
    (Utilities|Casting|CastToCharacter _returnvalue)
    (Pawn|Input|AddMovementInput (Variables|/Script/Engine.Actor|GetInstigator _returnvalue) (Math|Vector|Normalize (- (.worldlocation _value) (Transformation|GetActorLocation _returnvalue))) 1.0 false)
    (Movement|TurntoFace)
    ;[1 1 1] Remove node if reached
    (if (Utilities|Operators|EqualEqual (Transformation|GetActorLocation (Components|GetOwner)) (.worldlocation _value) (Variables|Default|GetAcceptanceRadius))
      (Utilities|Array|RemoveIndex (Variables|Default|GetPath)))))

(fn TurntoFace
  (bind _returnvalue (Components|GetOwner))
  (bind _returnvalue_2 (Transformation|GetActorLocation _returnvalue))
  (bind _instigator (Variables|/Script/Engine.Actor|GetInstigator _returnvalue))
  (bind _returnvalue_3 (Class|Pawn|GetLastMovementInputVector _instigator))
  (bind _returnvalue_4 (* 5e+01 _returnvalue_3))
  (bind _returnvalue_5 (+ _returnvalue_2 _returnvalue_4))
  (Utilities|Casting|CastToCharacter _returnvalue)
  (Transformation|SetActorRotation _returnvalue (Math|Rotator|FindLookatRotation _returnvalue_2 (Math|Vector|MakeVector (.x _returnvalue_5) (.y _returnvalue_5) 88.0))))

(fn SetTargetPath
  (params (Target :type Vector))
  ;[1 1 1] Function calls the change path event
  (CallFunction|ChangePath Target))

(fn UpdateDynamicNodes
  (for _array_element (Variables|/Game/GardenOfMedusa/Blueprints/Pathfinding/BP_Grid.BP_Grid_C|GetInconsistentNodes (Variables|Default|GetGrid))
    ;[1 1 1] Check if any node costs changed, and add to array if there is change
    (if (!= (.nodecost (.Value (Utilities|Map|Find (Variables|/Game/GardenOfMedusa/Blueprints/Pathfinding/BP_Grid.BP_Grid_C|GetNodes (Variables|Default|GetGrid)) _array_element))) (.nodecost (.Value (Utilities|Map|Find (Variables|Default|GetNodes) _array_element))))
      (Utilities|Array|AddUnique (LocalVariables|GetChangedNodes) _array_element)
      ;[1 1 1] Update the pathfinder's inconsistent nodes from the grid
      (Utilities|Map|Add (Variables|Default|GetNodes) _array_element (Utilities|Struct|MakeStruct_Node (.groundtype (.Value (Utilities|Map|Find (Variables|/Game/GardenOfMedusa/Blueprints/Pathfinding/BP_Grid.BP_Grid_C|GetNodes (Variables|Default|GetGrid)) _array_element))) (.worldlocation (.Value (Utilities|Map|Find (Variables|/Game/GardenOfMedusa/Blueprints/Pathfinding/BP_Grid.BP_Grid_C|GetNodes (Variables|Default|GetGrid)) _array_element))) (.gridindex (.Value (Utilities|Map|Find (Variables|/Game/GardenOfMedusa/Blueprints/Pathfinding/BP_Grid.BP_Grid_C|GetNodes (Variables|Default|GetGrid)) _array_element))) (.nodecost (.Value (Utilities|Map|Find (Variables|/Game/GardenOfMedusa/Blueprints/Pathfinding/BP_Grid.BP_Grid_C|GetNodes (Variables|Default|GetGrid)) _array_element))) 0 0 0 "(X=0.000000,Y=0.000000)"))))
  (Pathfinding|CheckifPathNeedsChange (LocalVariables|GetChangedNodes)))

(fn CheckifPathNeedsChange
  (params (Changed%20Nodes :type Array%20of%20Vector%202D%20Structures))
  ;[1 1 1] Iterate through changed nodes to see if it affected path
  (for _array_element Changed%20Nodes
    (LocalVariables|SetPathChanged (Utilities|Array|ContainsItem (Variables|Default|GetPath) _array_element)))
  ;[1 1 1] If the direct path changed, then set the path with new node weights
  (if (LocalVariables|GetPathChanged)
    (bind _asbp_medusa (Utilities|Casting|CastToBP_Medusa (Components|GetOwner)))
    (Movement|SetTargetPath (Math|Conversions|ToVector(Vector2D) (Variables|/Game/GardenOfMedusa/Blueprints/Characters/BP_Medusa.BP_Medusa_C|GetTarget _asbp_medusa)))))

(fn GetNodeinNavigableRadius
  (params (Center :type Vector) (Radius :type Float%20%28double-precision%29))
  ;[1 1 1] Init Center and Radius from inputs
  (LocalVariables|SetCenterL Center)
  (LocalVariables|SetRadiusL Radius)
  ;[1 1 1] Calculate a random angle between 0 and 2 PI
  (LocalVariables|SetTheta (* (Math|Random|RandomFloat) (* (Math|Trig|GetPI) 2.0)))
  ;[1 1 1] Calculate random radial value within circle's radius
  (LocalVariables|SetRadialValue (* (LocalVariables|GetRadiusL) (Math|Float|Sqrt (Math|Random|RandomFloat))))
  ;[1 1 1] Calculate the random X and Y coordinates
  (LocalVariables|SetX (* (+ (.X (Math|Vector|BreakVector (LocalVariables|GetCenterL))) (LocalVariables|GetRadialValue)) (Math|Trig|Cos(Radians) (LocalVariables|GetTheta))))
  (LocalVariables|SetY (* (+ (.Y (Math|Vector|BreakVector (LocalVariables|GetCenterL))) (LocalVariables|GetRadialValue)) (Math|Trig|Sin(Radians) (LocalVariables|GetTheta))))
  ;[1 1 1] Get the node from the calculated coordinates and check if navigable
  (if (<= (.nodecost (Default|GetNodefromWorldPosition (Variables|Default|GetGrid) (Math|Vector2D|MakeVector2D (LocalVariables|GetX) (LocalVariables|GetY)))) 1) ; Call recursively if not navigable
    (return (.worldlocation (Default|GetNodefromWorldPosition (Variables|Default|GetGrid) (Math|Vector2D|MakeVector2D (LocalVariables|GetX) (LocalVariables|GetY)))))
    (else
      ;[1 1 1] Recursive Call
      (bind _out_location (Pathfinding|GetNodeinNavigableRadius (LocalVariables|GetCenterL) (LocalVariables|GetRadiusL)))
      (return _out_location))))