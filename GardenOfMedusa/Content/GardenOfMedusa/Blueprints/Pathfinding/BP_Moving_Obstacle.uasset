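; BP_Moving_Obstacle is a pathfinding obstacle in Garden of Medusa that can switch between open and closed.
; ToggleObstacle flips IsOpen and has the Grid check its inconsistent nodes.
; A chain that toggles it and updates BP_Medusa's Pathfinder dynamic nodes is disconnected, so BeginPlay only runs a delay with no follow-up.
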(event EventBeginPlay
  (Utilities|FlowControl|Delay 3.0))

(event Collision|EventActorBeginOverlap
  (params (OtherActor :type Actor%20Object%20Reference)))

(event EventTick
  (params (DeltaSeconds :type Float%20%28single-precision%29)))

(fn ConstructionScript)

(fn ToggleObstacle
  ;[1 1 1] Toggle the weights of the nodes affected by the obstacle, and then have the grid check its nodes
  (Variables|Default|SetIsOpen (not (Variables|Default|GetIsOpen)))
  (Default|CheckInconsistentNodes (Variables|Default|GetGrid)))