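; Blueprint function library that implements a priority queue of grid node keys for cost-based pathfinding in Garden of Medusa.
; Push adds a key without duplicates and calls Sort, while Pop removes and returns the front key with the updated queue.
; Sort is a bubble sort that looks up each node in the grid, ordering by lowest final cost and breaking ties on estimated cost to target.
; GetSize and IsEmpty report on the array length.
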(fn Push
  (params (Queue :type Struct%20Priority%20Queue%20Structure) (NodeKey :type Vector%202D%20Structure) (Grid :type BP%20Grid%20Object%20Reference))
  ;[1 1 1] Push node to back of the queue and then sort it
  (LocalVariables|SetPriorityQueue Queue)
  (Utilities|Array|AddUnique (Utilities|Struct|BreakStruct_PriorityQueue (LocalVariables|GetPriorityQueue)) NodeKey)
  (bind _structout (Utilities|Struct|SetmembersinStruct_PriorityQueue (LocalVariables|GetPriorityQueue)))
  (PriorityQueue|Sort _structout Grid Grid)
  (return _structout))

(fn Pop
  (params (Queue :type Struct%20Priority%20Queue%20Structure))
  ;[1 1 1] Remove the node at the front of the queue and return it as a copy
  (LocalVariables|SetPriorityQueue Queue)
  (LocalVariables|SetReturn%20Node (Utilities|Array|Get(acopy) (.nodearray (LocalVariables|GetPriorityQueue))))
  (Utilities|Array|RemoveIndex (Utilities|Struct|BreakStruct_PriorityQueue (LocalVariables|GetPriorityQueue)))
  (Utilities|Struct|SetmembersinStruct_PriorityQueue (LocalVariables|GetPriorityQueue))
  (return (LocalVariables|GetReturn%20Node) (LocalVariables|GetPriorityQueue)))

(fn Sort
  (params (Queue :type Struct%20Priority%20Queue%20Structure) (Grid :type BP%20Grid%20Object%20Reference))
  ;[1 1 1] Double loop to iterate through the array multiple times. This ensures multiple passes for sorting if needed
  (LocalVariables|SetNodeGrid Grid)
  (LocalVariables|SetPriorityQueue Queue)
  (for _index (range 0 (- (Utilities|Array|Length (.nodearray (LocalVariables|GetPriorityQueue))) 1))
    (LocalVariables|SetSwapped false)
    (for _index_2 (range 0 (- (- (Utilities|Array|Length (.nodearray (LocalVariables|GetPriorityQueue))) _index) 1))
      ;[1 1 1] Set the checked indices
      (LocalVariables|SetCheckIndex _index_2)
      (LocalVariables|SetCheckNextIndex (Math|Integer|%(Integer) (+ _index_2 1) (Utilities|Array|Length (.nodearray (LocalVariables|GetPriorityQueue)))))
      (if (> (.finalcost (.Value (Utilities|Map|Find (Variables|/Game/GardenOfMedusa/Blueprints/Pathfinding/BP_Grid.BP_Grid_C|GetNodes (LocalVariables|GetNodeGrid)) (Utilities|Array|Get(acopy) (.nodearray (LocalVariables|GetPriorityQueue)) (LocalVariables|GetCheckIndex))))) (.finalcost (.Value (Utilities|Map|Find (Variables|/Game/GardenOfMedusa/Blueprints/Pathfinding/BP_Grid.BP_Grid_C|GetNodes (LocalVariables|GetNodeGrid)) (Utilities|Array|Get(acopy) (.nodearray (LocalVariables|GetPriorityQueue)) (LocalVariables|GetCheckNextIndex))))))
        ;[1 1 1] If the fCost on the left is bigger, swap the two
        (Utilities|Array|Swap (.nodearray (LocalVariables|GetPriorityQueue)) (LocalVariables|GetCheckIndex) (LocalVariables|GetCheckNextIndex))
        (LocalVariables|SetSwapped true)
        (elif (== (.finalcost (.Value (Utilities|Map|Find (Variables|/Game/GardenOfMedusa/Blueprints/Pathfinding/BP_Grid.BP_Grid_C|GetNodes (LocalVariables|GetNodeGrid)) (Utilities|Array|Get(acopy) (.nodearray (LocalVariables|GetPriorityQueue)) (LocalVariables|GetCheckNextIndex))))) (.finalcost (.Value (Utilities|Map|Find (Variables|/Game/GardenOfMedusa/Blueprints/Pathfinding/BP_Grid.BP_Grid_C|GetNodes (LocalVariables|GetNodeGrid)) (Utilities|Array|Get(acopy) (.nodearray (LocalVariables|GetPriorityQueue)) (LocalVariables|GetCheckIndex)))))) ; fCosts are equal
          ;[1 1 1] If the hCost on the left is bigger, swap the two.
          (if (> (.estimatedcosttotarget (.Value (Utilities|Map|Find (Variables|/Game/GardenOfMedusa/Blueprints/Pathfinding/BP_Grid.BP_Grid_C|GetNodes (LocalVariables|GetNodeGrid)) (Utilities|Array|Get(acopy) (.nodearray (LocalVariables|GetPriorityQueue)) (LocalVariables|GetCheckIndex))))) (.estimatedcosttotarget (.Value (Utilities|Map|Find (Variables|/Game/GardenOfMedusa/Blueprints/Pathfinding/BP_Grid.BP_Grid_C|GetNodes (LocalVariables|GetNodeGrid)) (Utilities|Array|Get(acopy) (.nodearray (LocalVariables|GetPriorityQueue)) (LocalVariables|GetCheckNextIndex))))))
            (Utilities|Array|Swap (.nodearray (LocalVariables|GetPriorityQueue)) (LocalVariables|GetCheckIndex) (LocalVariables|GetCheckNextIndex))
            (LocalVariables|SetSwapped true))))))
  ;[1 1 1] If one pass goes through and nothing was swapped, the array is now sorted and can be returned.
  (if (not (LocalVariables|GetSwapped))
    (return (LocalVariables|GetPriorityQueue))))

(fn GetSize
  (params (Queue :type Struct%20Priority%20Queue%20Structure))
  ;[1 1 1] Return the length of the array as the queue's size
  (return (Utilities|Array|Length (.nodearray Queue))))

(fn IsEmpty
  (params (Queue :type Struct%20Priority%20Queue%20Structure))
  (return (not (> (PriorityQueue|GetSize Queue) 0))))