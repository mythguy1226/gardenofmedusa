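; BP_ShiftingWall is a maze wall obstacle that shifts vertically between open and closed states.
; ShiftWall waits briefly, then reverses or plays the MoveObstacle timeline depending on IsOpen, setting the root's height from the curve scaled by the actor's Z scale.
; When the timeline finishes, it toggles the obstacle state and has BP_Medusa's Pathfinder update its dynamic nodes to account for the change.
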(event Custom|ShiftWall
  (bind _returnvalue (Transformation|GetActorLocation))
  ;[1 1 1] Small delay and check on obstacle state
  (Utilities|FlowControl|Delay 0.2)
  (if (Variables|Default|GetIsOpen)
    ;[1 1 1] Update wall location while shifting
    (bind _movement (Timeline|MoveObstacle Reverse)
      (:Update
        (Transformation|SetRelativeLocation (Variables|Default|GetDefaultSceneRoot) (Math|Vector|MakeVector (.x _returnvalue) (.y _returnvalue) (* (.z _movement) (.z (Transformation|GetActorScale3D)))) false false))
      (:Finished
        ;[1 1 1] When wall is done shifting, update obstacle state and grid nodes
        (CallFunction|ToggleObstacle)
        (bind _returnvalue_2 (Actor|GetActorOfClass "/Game/GardenOfMedusa/Blueprints/Characters/BP_Medusa.BP_Medusa_C"))
        (Default|UpdateDynamicNodes (Variables|/Game/GardenOfMedusa/Blueprints/Characters/BP_Medusa.BP_Medusa_C|GetPathfinder _returnvalue_2))))
    (else
      (Timeline|MoveObstacle Play))))

(fn ConstructionScript
  (|CallParentFunction))